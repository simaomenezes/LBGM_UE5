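; Base area-of-effect actor for the damage system that finds pawns within a sphere around itself and reports each one.
; Trigger runs the sphere overlap, either when called or automatically shortly after BeginPlay if enabled, optionally ignoring the instigator.
; Each hit fires the OnAOEOverlapActor dispatcher and prints the actor name, leaving the effect itself to listeners.
; An optional debug sphere shows the affected radius.
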(event Custom|SpawnAOESphere
  ;[0.1338 0 0.15 0.5] Draw Debug - Sphere
  (if (Variables|Default|GetDrawDebugSphere)
    (Rendering|Debug|DrawDebugSphere (Transformation|GetActorLocation) (Variables|Default|GetSphereRadius) 12 "(R=1.000000,G=0.000000,B=0.770756,A=1.000000)" 2.0 1.0))
  (bind _outactors (Collision|SphereOverlapActors (Transformation|GetActorLocation) (Variables|Default|GetSphereRadius) (Utilities|Array|MakeArray "ObjectTypeQuery3") 0 (select (Variables|Default|GetIgnoreInstagator) (Utilities|Array|MakeArray (Game|GetInstigator)) 0)))
  (for _array_element _outactors
    (Default|CallOnAOEOverlapActor _array_element)
    (Development|PrintString (Utilities|GetDisplayName _array_element))))

(event Custom|Trigger
  (CallFunction|SpawnAOESphere))

(event EventBeginPlay
  (if (Variables|Default|GetTriggerBeginPlay)
    (Utilities|FlowControl|Delay 0.2)
    (CallFunction|Trigger)))

(fn ConstructionScript)