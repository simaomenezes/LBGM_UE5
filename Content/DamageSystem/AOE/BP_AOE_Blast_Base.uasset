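; Base blast area-of-effect actor in the damage system, adding visual and audio feedback to its parent's Trigger behavior.
; On Trigger it runs the parent logic, spawns the blast particle effect attached to its root, and plays the blast sound at its location.
; Without a valid effect it destroys itself after a short delay.
; The destroy-on-particle-finished binding is unconnected, so actors with an effect are not destroyed here.
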(event Custom|SystemFinished
  (params (PSystem :type Particle%20System%20Component%20Object%20Reference))
  ;[0 0.008795 0.15 0.5] Spawn Blast Effect flow
  (Actor|DestroyActor))

(event Custom|SpawnBlastEffect
  ;[0 0.008795 0.15 0.5] Spawn Blast Effect flow
  (bind _blasteffect (Variables|Default|GetBlasTEffect)
    (:then
      (bind _returnvalue (Effects|SpawnEmitterAttached _blasteffect (Variables|Default|GetDefaultSceneRoot) "None")))
    (:else
      (Utilities|FlowControl|Delay 1.0)
      (Actor|DestroyActor))))

(event Custom|PlayBlastSound
  ;[0.15 0.15 0.15 0.5] Play Sound for Blast Effect
  (bind _blastsound (Variables|Default|GetBlastSound)
    (:then
      (Audio|PlaySoundatLocation _blastsound (Transformation|GetActorLocation) "0, 0, 0" 1.0 1.0 0.0 0 0 0 0))
    (:else)))

(event EventBeginPlay
  (|CallParentFunction) ; This node is disabled and will not be called.\nDrag off pins to build functionality.
)

(event Collision|EventActorBeginOverlap
  (params (OtherActor :type Actor%20Object%20Reference)))

(event EventTick
  (params (DeltaSeconds :type Float%20%28single-precision%29)))

(event EventTrigger
  (|CallParentFunction)
  (CallFunction|SpawnBlastEffect)
  (CallFunction|PlayBlastSound))

(fn ConstructionScript
  (|CallParentFunction))