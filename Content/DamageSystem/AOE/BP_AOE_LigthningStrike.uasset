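; Lightning strike area-of-effect actor that marks its location with a ground decal before striking.
; On BeginPlay it runs parent logic, spawns the warning decal, waits DelayBeforeStrike, then calls Trigger, which is not defined in this graph.
; After triggering, it checks that the decal is valid but destroys DefaultSceneRoot rather than the decal component.
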(event Collision|EventActorBeginOverlap
  (params (OtherActor :type Actor%20Object%20Reference))
  (|CallParentFunction OtherActor) ; This node is disabled and will not be called.\nDrag off pins to build functionality.
)

(event EventTick
  (params (DeltaSeconds :type Float%20%28single-precision%29))
  (|CallParentFunction DeltaSeconds) ; This node is disabled and will not be called.\nDrag off pins to build functionality.
)

(event EventBeginPlay
  (|CallParentFunction)
  (bind _returnvalue (Rendering|Decal|SpawnDecalatLocation "/Game/KTP_Effect/Materials/M_botton11_1.M_botton11_1" "25.000000,256.000000,256.000000" (Transformation|GetActorLocation) "-90.000000,0.000000,0.000000" 0.0))
  (Utilities|FlowControl|Delay (Variables|Default|GetDelayBeforeStrike))
  (CallFunction|Trigger)
  (Utilities|IsValid _returnvalue
    (:Is%20Valid
      (Components|DestroyComponent (Variables|Default|GetDefaultSceneRoot)))))

(fn ConstructionScript
  (|CallParentFunction))