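; Player interaction component for a Character that lets it interact with nearby actors implementing BPI_Interactable.
; Capsule overlap begin and end events maintain a list of interactables in range.
; The IA_Interact input plays the AM_ItemPickup montage and sends Interact to the first listed actor, both as the montage starts and on its "Interact" notify.
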(event Custom|HandleCapsuleOverlapBegin
  (params (OverlappedComponent :type Primitive%20Component%20Object%20Reference) (OtherActor :type Actor%20Object%20Reference) (OtherComp :type Primitive%20Component%20Object%20Reference) (OtherBodyIndex :type Integer) (bFromSweep :type Boolean) (SweepResult :type Hit%20Result%20Structure%20%28by%20ref%29))
  (if (Utilities|DoesObjectImplementInterface OtherActor "/Game/InteractionSystem/BP_Interfaces/BPI_Interactable.BPI_Interactable_C")
    (Utilities|Array|AddUnique (Variables|Default|GetInteractablesInRanges) OtherActor)))

(event Custom|HandleCapsuleOverlapEnd
  (params (OverlappedComponent :type Primitive%20Component%20Object%20Reference) (OtherActor :type Actor%20Object%20Reference) (OtherComp :type Primitive%20Component%20Object%20Reference) (OtherBodyIndex :type Integer))
  (if (Utilities|DoesObjectImplementInterface OtherActor "/Game/InteractionSystem/BP_Interfaces/BPI_Interactable.BPI_Interactable_C")
    (Utilities|Array|RemoveItem (Variables|Default|GetInteractablesInRanges) OtherActor)))

(event Input|EnhancedActionEvents|EnhancedInputActionIA_Interact
  (params (ActionValue :type Boolean) (ElapsedSeconds :type Float%20%28double-precision%29) (TriggeredSeconds :type Float%20%28double-precision%29) (InputAction :type Input%20Action%20Object%20Reference :default "/Game/ThirdPerson/Input/Actions/IA_Interact.IA_Interact"))
  ;[1 0.7945 0.09375 0.5] Call flow to start interaction with any
  (:Started
    (if (Utilities|Array|IsNotEmpty (Variables|Default|GetInteractablesInRanges))
      (bind _notifyname (Animation|Montage|PlayMontage (Variables|/Script/Engine.Character|GetMesh (Variables|Default|GetCharacterRef)) "/Game/InteractionSystem/AnimMontage/Interact/AM_ItemPickup.AM_ItemPickup")
        (:then
          (Class|BPIInteractable|Interact(Message) (Utilities|Array|Get(acopy) (Variables|Default|GetInteractablesInRanges)) (Components|GetOwner) :!label _label))
        (:OnNotifyBegin
          (if (== _notifyname "Interact")
            (goto _label)))))))

(event EventBeginPlay
  (bind _ascharacter (Utilities|Casting|CastToCharacter (Components|GetOwner)))
  (Variables|Default|SetCharacterRef _ascharacter)
  (Collision|BindEventtoOnComponentBeginOverlap (Variables|/Script/Engine.Character|GetCapsuleComponent _ascharacter) (EventDispatchers|CreateEvent :!event Custom|HandleCapsuleOverlapBegin))
  (Collision|BindEventtoOnComponentEndOverlap (Variables|/Script/Engine.Character|GetCapsuleComponent _ascharacter) (EventDispatchers|CreateEvent :!event Custom|HandleCapsuleOverlapEnd)))