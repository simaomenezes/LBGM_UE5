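; BP_NPC is an interactable NPC in the interaction system that shows a "To Talk" prompt.
; On Interact, it rotates to the yaw that faces the interactor and plays a sound cue at its location.
; It reports a zero hold duration and the first interaction type enumerator, and contains no dialogue logic.
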(event EventInteract
  (params (Interactor :type Actor%20Object%20Reference))
  (Transformation|SetActorRotation (Math|Rotator|MakeRotator 0.0 0.0 (.yaw (Math|Rotator|FindLookatRotation (Transformation|GetActorLocation) (Transformation|GetActorLocation Interactor)))))
  (Audio|PlaySoundatLocation "/Game/Liminal_Pools_001/Cues/juanjo_sound_Pool_0009_Cue.juanjo_sound_Pool_0009_Cue" (Transformation|GetActorLocation) "0, 0, 0" 1.0 1.0 0.0 0 0 0 0))

(fn ConstructionScript)

(fn GetHoldDuration
  (return 0.0))

(fn GetInteractionPrompt
  (return "To Talk"))

(fn GetInteractionType
  (return "NewEnumerator0"))