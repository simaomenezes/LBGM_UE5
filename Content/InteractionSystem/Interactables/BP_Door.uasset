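; BP_Door is an interactable door that swings open and shut through the interaction system, supplying its own prompt, type and zero hold duration.
; Interact branches on IsOpen to call OpenDoor or CloseDoor, which play or reverse a timeline driving the Door's yaw.
; IsOpen reads inverted: OpenDoor clears it and CloseDoor sets it, while the prompt offers "close" when it is true.
; Interact also prints IsOpen on each use.
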(event Custom|CloseDoor
  (Variables|Default|SetIsOpen true)
  ;[0.15 0.15 0.15 0.5] Making animation to door
  (bind _zrotation (Timeline|OpenDoorTimeLine Reverse)
    (:Update
      (Transformation|SetRelativeRotation (Variables|Default|GetDoor) (Math|Rotator|MakeRotator 0.0 0.0 _zrotation) false false))))

(event Custom|OpenDoor
  (Variables|Default|SetIsOpen false)
  ;[0.15 0.15 0.15 0.5] Making animation to door
  (bind _zrotation (Timeline|OpenDoorTimeLine Play)
    (:Update
      (Transformation|SetRelativeRotation (Variables|Default|GetDoor) (Math|Rotator|MakeRotator 0.0 0.0 _zrotation) false false))))

(event EventInteract
  (params (Interactor :type Actor%20Object%20Reference))
  (bind _isopen (Variables|Default|GetIsOpen))
  (if _isopen
    (Development|PrintString (Utilities|String|ToString(Boolean) _isopen))
    (CallFunction|OpenDoor)
    (else
      (Development|PrintString (Utilities|String|ToString(Boolean) _isopen))
      (CallFunction|CloseDoor))))

(fn ConstructionScript)

(fn GetHoldDuration
  (return 0.0))

(fn GetInteractionPrompt
  (return (Utilities|String|SelectText "to close the door" "to open the door" (Variables|Default|GetIsOpen))))

(fn GetInteractionType
  (return "NewEnumerator0"))