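; Base pickup item actor for the interaction system, removed from the level when an actor interacts with it.
; Interact only prints an "added to inventory" message with the item and interactor names, without storing anything in an inventory.
; It then plays an explosion sound at its location and destroys itself after a short delay.
; GetInteractionType exposes the item's InteractionType variable to callers.
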(event EventInteract
  (params (Interactor :type Actor%20Object%20Reference))
  (Development|PrintString (Utilities|String|ToString(Text) (Utilities|Text|FormatText "Added {ItemName} to the inventory of {ActorName}" (Utilities|GetDisplayName self) (Utilities|GetDisplayName Interactor))))
  (Audio|PlaySoundatLocation "/Game/StarterContent/Audio/Explosion01.Explosion01" (Transformation|GetActorLocation) "0, 0, 0" 1.0 1.0 0.0 0 0 0 0)
  (Utilities|FlowControl|Delay 0.5)
  (Actor|DestroyActor))

(fn ConstructionScript)

(fn GetInteractionType
  (return (Variables|Default|GetInteractionType)))